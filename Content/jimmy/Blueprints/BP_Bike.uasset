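; Bike Blueprint using Chaos Vehicle movement that drives dust trail effects on its front and back wheels.
; Every Tick, DustTrail reads the absolute forward speed, activating both wheel effects while moving and deactivating them at a standstill.
; While active, a clamped remap of speed feeds each effect's WheelSpeed parameter.
; The speed is also printed every frame as debug output.
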(event Custom|Dust%20Trail
  (bind _chaosvehiclemovement (Variables|Default|GetChaosVehicleMovement))
  (bind _wheel_fx_back (Variables|Default|Getwheel%20FX%20Back))
  (bind _returnvalue (Vehicle|GetForwardSpeed _chaosvehiclemovement))
  (bind _returnvalue_2 (Math|Conversions|ToVector(Float) _returnvalue))
  (bind _returnvalue_3 (Math|Vector|VectorLength _returnvalue_2))
  (bind _returnvalue_4 (Math|Float|Absolute(Float) _returnvalue_3))
  (Development|PrintString (Utilities|String|ToString(Float) _returnvalue_4))
  (if (> _returnvalue_4 0.0)
    (Components|Activation|SetActive _wheel_fx_back true false)
    (Effects|Components|ParticleSystem|SetFloatParameter (Variables|Default|Getwheel%20FX%20Front) "WheelSpeed" (Math|Float|MapRangeClamped _returnvalue_3 0.0 1e+03 0.1 1.0))
    (else
      (Components|Activation|Deactivate _wheel_fx_back))))

(event EventBeginPlay)

(event Collision|EventActorBeginOverlap
  (params (OtherActor :type Actor%20Object%20Reference)))

(event EventTick
  (params (DeltaSeconds :type Float%20%28single-precision%29))
  (CallFunction|DustTrail))

(fn ConstructionScript)