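; BP_Bike is a bike Blueprint with a Chaos vehicle movement component and dust trail effects on its front and back wheels.
; Every Tick, it maps forward speed in MPH through a clamped range into the WheelSpeed parameter of both wheel effects, keeping a small minimum value.
; Tick also prints the current steering input as debug output, while a speed printout is left unconnected.
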(event Custom|Dust%20Trail
  ;[1 1 1] Wheel FX
  (Effects|Components|ParticleSystem|SetFloatParameter (Variables|Default|Getwheel%20FX%20Front) "WheelSpeed" (Math|Float|MapRangeClamped (Class|ChaosVehicleMovementComponent|GetForwardSpeedMPH (Variables|Default|GetChaosVehicleMovement)) 0.0 2e+01 0.1 1.0)))

(event EventBeginPlay)

(event Collision|EventActorBeginOverlap
  (params (OtherActor :type Actor%20Object%20Reference)))

(event EventTick
  (params (DeltaSeconds :type Float%20%28single-precision%29))
  (CallFunction|DustTrail)
  (bind _returnvalue (Class|ChaosVehicleMovementComponent|GetSteeringInput (Variables|Default|GetChaosVehicleMovement)))
  (Development|PrintString (Utilities|String|ToString(Float) _returnvalue)))

(fn ConstructionScript)