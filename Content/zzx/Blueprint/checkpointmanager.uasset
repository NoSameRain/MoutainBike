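; Checkpoint manager actor that makes the level's checkpoints activate one after another in order.
; On BeginPlay it gathers all checkpoints, registers itself on each, sorts them by their Ratio value, assigns indices and activates the first.
; Sorting orders a copy of the ratios and maps them back to the original array positions.
; Notifycheckpoint accepts only the current index, then advances and activates the next checkpoint until the last.
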(event Collision|EventActorBeginOverlap
  (params (OtherActor :type Actor%20Object%20Reference)))

(event EventTick
  (params (DeltaSeconds :type Float%20%28single-precision%29)))

(event EventBeginPlay
  (bind _outactors (Actor|GetAllActorsOfClass "/Game/zzx/Blueprint/checkpoints.checkpoints_C"))
  (Variables|Default|Setcheckpoints _outactors)
  (for _array_element (Variables|Default|Getcheckpoints)
    (Variables|/Game/zzx/Blueprint/checkpoints.checkpoints_C|Setrecheckpointmanager _array_element self)
    (Utilities|Array|Add (Variables|Components|Getratioarray) (Variables|/Game/zzx/Blueprint/checkpoints.checkpoints_C|Getratio _array_element)))
  (bind _return_checkpoints (CallFunction|Sortbyratio))
  (Variables|Default|Setcheckpoints _return_checkpoints)
  (for (_array_element_2 _array_index) (Variables|Default|Getcheckpoints)
    (Variables|/Game/zzx/Blueprint/checkpoints.checkpoints_C|SetIndex _array_element_2 _array_index)
    (bind _output_get (Variables|/Game/zzx/Blueprint/checkpoints.checkpoints_C|SetIsactivited (Utilities|Array|Get(acopy) (Variables|Default|Getcheckpoints)) true))
    (Default|Setactive (Utilities|Array|Get(acopy) (Variables|Default|Getcheckpoints)) _output_get))
  (Development|PrintString "Hello"))

(fn ConstructionScript)

(fn Activatecheckpoint
  (params (index :type Integer))
  (Default|Setactive (Utilities|Array|Get(acopy) (Variables|Default|Getcheckpoints) index) true))

(fn Notifycheckpoint
  (params (index :type Integer))
  (if (and (== index (Variables|Default|Geti)) (<= (+ (Variables|Default|Geti) 2) (Utilities|Array|Length (Variables|Default|Getcheckpoints))))
    (bind _output_get (Variables|Default|Seti (+ (Variables|Default|Geti) 1)))
    (CallFunction|Activatecheckpoint _output_get)
    (Development|PrintString "Check point Reached")))

(fn Sortbyratio
  (LocalVariables|Setoldratioarray (Variables|Components|Getratioarray))
  (Class|KismetArrayLibrary|SortFloatArray (Variables|Components|Getratioarray))
  (for _array_element (Variables|Components|Getratioarray)
    (for (_array_element_2 _array_index) (LocalVariables|Getoldratioarray)
      (if (== _array_element_2 _array_element)
        (Utilities|Array|Add (Variables|Components|Getindexarray) _array_index))))
  (for _array_element_3 (Variables|Components|Getindexarray)
    (Utilities|Array|Add (LocalVariables|Getsorted%20checkpoints) (Utilities|Array|Get(acopy) (Variables|Default|Getcheckpoints) _array_element_3)))
  (return (LocalVariables|Getsorted%20checkpoints)))