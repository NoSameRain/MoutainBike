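; Checkpoint actor for a bike race that records a respawn point when a BP_Bike passes through its collision box.
; On BeginPlay it hides itself and computes its normalized distance along the first spline actor found in the level.
; On overlap it writes its location and rotation to the bike, plays a sound, deactivates and notifies the checkpoint manager with its index.
; Setactive toggles both collision and mesh visibility.
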(event OnComponentBeginOverlap(CollisionBox)
  (params (OverlappedComponent :type Primitive%20Component%20Object%20Reference) (OtherActor :type Actor%20Object%20Reference) (OtherComp :type Primitive%20Component%20Object%20Reference) (OtherBodyIndex :type Integer) (bFromSweep :type Boolean) (SweepResult :type Hit%20Result%20Structure%20%28by%20ref%29))
  (bind _collisionbox (Variables|Default|GetCollisionBox))
  (Development|PrintString "Overlapped")
  (bind _asbp_bike (Utilities|Casting|CastToBP_Bike OtherActor))
  (Variables|/Script/Bike.BikePawn|SetLastCheckPointLocation _asbp_bike (Transformation|GetWorldLocation _collisionbox))
  (Variables|/Script/Bike.BikePawn|SetLastCheckPointRotation _asbp_bike (Transformation|GetWorldRotation _collisionbox))
  (Variables|/Script/Bike.BikePawn|SetreachedCheckPoint _asbp_bike true)
  (Audio|PlaySound2D 0 1.0 1.0 0.0 0 0)
  (bind _output_get (Variables|Default|SetIsactivited false))
  (CallFunction|Setactive _output_get)
  (Default|Notifycheckpoint (Variables|Default|Getrecheckpointmanager) (Variables|Default|GetIndex)))

(event EventBeginPlay
  (CallFunction|Setactive false)
  (bind _outactors (Actor|GetAllActorsOfClass "/Game/zzx/Blueprint/spline.spline_C"))
  (Variables|Default|Setratio (/ (Class|SplineComponent|GetDistanceAlongSplineatLocation (Variables|/Game/zzx/Blueprint/spline.spline_C|GetSpline (Utilities|Array|Get(acopy) _outactors)) (Class|SplineComponent|GetLocationatSplineInputKey (Variables|/Game/zzx/Blueprint/spline.spline_C|GetSpline (Utilities|Array|Get(acopy) _outactors)) (Class|SplineComponent|FindInputKeyClosesttoWorldLocation (Variables|/Game/zzx/Blueprint/spline.spline_C|GetSpline (Utilities|Array|Get(acopy) _outactors)) (Transformation|GetWorldLocation (Variables|Default|GetStaticMesh))) "World") "World") (Spline|GetSplineLength (Variables|/Game/zzx/Blueprint/spline.spline_C|GetSpline (Utilities|Array|Get(acopy) _outactors))))))

(event Collision|EventActorBeginOverlap
  (params (OtherActor :type Actor%20Object%20Reference)))

(event EventTick
  (params (DeltaSeconds :type Float%20%28single-precision%29)))

(fn ConstructionScript)

(fn Setactive
  (params (isactived :type Boolean))
  (bind _collisionbox (Variables|Default|GetCollisionBox))
  (if isactived
    (Collision|SetCollisionEnabled _collisionbox "QueryAndPhysics")
    (Rendering|SetVisibility (Variables|Default|GetStaticMesh) true true)
    (else
      (Collision|SetCollisionEnabled _collisionbox "NoCollision")
      (Rendering|SetVisibility (Variables|Default|GetStaticMesh) false true))))